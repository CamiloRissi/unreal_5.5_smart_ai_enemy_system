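; Ranged enemy Blueprint that fights with a rifle, overriding parent enemy behavior for weapon, attack, movement speed and ideal range.
; On BeginPlay it spawns the rifle and attaches it to a hand socket.
; Attack plays the fire montage, whose notify has BPCAttacks fire a blockable bullet from weapon to target; completion or interruption calls AttackEnd.
; Movement states map to walk speeds, and attack and defend radii are fixed.
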(event `self.ReceiveBeginPlay`
  ; BeginPlay (Extend) Equip weapon on begin play
  (`parent.ReceiveBeginPlay`)
  (`/Game/Enemies/AI/BPI_EnemyAI.EquipWeapon`))

(event `/Game/Enemies/AI/BPI_EnemyAI.EquipWeapon`
  ; EquipWeapon (Override) This event will be called on begin play
  ;; Spawn the Weapon and attach it to the rifle socket. Also SET the weapon actor variable.
  (bind _returnvalue (`|SpawnActorFromClass` "/Game/Weapons/BP_Weapon_Rifle.BP_Weapon_Rifle_C" (`KismetMathLibrary.MakeTransform` (0.0 0.0 0.0)) "Undefined" "MultiplyWithRoot" null null))
  (bind _output_get (set `self.WeaponActor` _returnvalue))
  (bind _returnvalue_2 (`self.K2_AttachToComponent` _output_get (`self.Mesh`) "hand_r_rifle_socket" "SnapToTarget" "SnapToTarget" "SnapToTarget" true))
  ;; SET is wielding weapon to true
  (set `self.IsWieldingWeapon` _returnvalue_2)
  ;; Finally notify when completed (This call made by this enemy is not being expetec nowhere, but for good practice)
  (`self.OnWeaponEquipped`))

(event `/Game/Enemies/AI/BPI_EnemyAI.Attack`
  (params (AttackTarget :type "Actor Object Reference"))
  ; Event Attack (Extend)
  (`parent.Attack` AttackTarget)
  ;; Play Attack Montage. Call Attack End (Parent) after Montage completed or interrupted
  (bind _notifyname (`|PlayMontage` (`self.Mesh`) "/Game/Animations/Rifle/Montage_Rifle_Fire.Montage_Rifle_Fire")
    (:`OnCompleted`
      (`self.AttackEnd` AttackTarget :!label _label))
    (:`OnInterrupted`
      (goto _label))
    (:`OnNotifyBegin`
      ;; At the Montage Notify, Call Fire Bullet (BPC Attacks)
      (switch `name` _notifyname
        (:`Fire`
          (`/Game/Attacks/BPC_Attacks.FireBullet` (`self.BPC_Attacks`) (`self.K2_GetActorLocation` (`self.WeaponActor`)) (`self.K2_GetActorLocation` AttackTarget) (make `/Game/DamageSystem/S_DamageInfo` 15.0 "NewEnumerator2" "NewEnumerator0" false true)))))))

(fn `GetIdealRange`
  (returns (AttackRadius :type "Float (double-precision)") (DefendRadius :type "Float (double-precision)"))
  ; Get Ideal Range (Override)
  (return 600.0 600.0))

(fn `SetMovementSpeed`
  (params (Speed :type "/Game/Enemies/AI/Enums/E_MovementSpeed Enum" :default "NewEnumerator0"))
  (returns (SpeedValue :type "Float (double-precision)"))
  ; Set Movement Speed (Override)
  (set `CharacterMovementComponent.MaxWalkSpeed` (select `/Game/Enemies/AI/Enums/E_MovementSpeed` Speed :`NewEnumerator1` 200.0 :`NewEnumerator2` 300.0 :`NewEnumerator3` 500.0 :!type "Float (single-precision)") (`self.CharacterMovement`))
  (return 0.0))

(fn `UserConstructionScript`
  (`parent.UserConstructionScript`))