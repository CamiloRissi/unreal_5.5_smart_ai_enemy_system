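; Melee enemy Blueprint that extends its parent's attack and weapon events with sword combat, plus its own blocking logic.
; Montage notifies time the forward sphere-trace damage and the sword's spawn or destruction, while dispatchers report equip, unequip and block completion to Behavior Tree tasks.
; Attacks are uninterruptible through the damage system component, whose OnBlocked event switches blocking to a react montage via a state enum that guards against ending the block early.
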(event `self.ReceiveBeginPlay`
  ; BeginPlay (Extend)
  (`parent.ReceiveBeginPlay`))

(event `/Game/Enemies/AI/BPI_EnemyAI.Attack`
  (params (AttackTarget :type "Actor Object Reference"))
  (bind _returnvalue (`self.K2_GetActorLocation`))
  ; Event Attack (Extend)
  (`parent.Attack` AttackTarget)
  ;; Play Attack Montage and SET IsInterruptible to false while doing so. Call Attack End (Parent) after Montage completed or interrupted
  (bind _notifyname (`|PlayMontage` (`self.Mesh`) "/Game/Animations/Melee/Montage_Sword_Slash.Montage_Sword_Slash")
    (:`then`
      (set `/Game/DamageSystem/BPC_DamageSystem.IsInterruptible` false (`self.BPC_DamageSystem`)))
    (:`OnCompleted`
      (`self.AttackEnd` AttackTarget :!label _label)
      (set `/Game/DamageSystem/BPC_DamageSystem.IsInterruptible` true (`self.BPC_DamageSystem`)))
    (:`OnInterrupted`
      (goto _label))
    (:`OnNotifyBegin`
      (switch `name` _notifyname
        (:`Slash`
          ;; Trace Sphere for Pawns
          (bind (_outhit _returnvalue_2) (`KismetSystemLibrary.SphereTraceSingleForObjects` :`Start` _returnvalue :`End` (+ _returnvalue (* (`self.GetActorForwardVector`) 200.0)) :`Radius` 20.0 :`ObjectTypes` (`|MakeArray` "ObjectTypeQuery3" :!type "EObjectTypeQuery Enum") :`DrawDebugType` "ForDuration"))
          ;; If a Pawn was hit, Call its Take Damage function
          (if _returnvalue_2
            (message `/Game/DamageSystem/BPI_Damagable.TakeDamage` (`.HitActor` (`GameplayStatics.BreakHitResult` _outhit)) (make `/Game/DamageSystem/S_DamageInfo` 25.0 "NewEnumerator1") self)))))))

(event `/Game/Enemies/AI/BPI_EnemyAI.EquipWeapon`
  ; EquipWeapon (Override) This event will be called by the BTT Equip Weapon
  ;; Play Montage, and when completed, notify the BTT
  (bind _notifyname (`|PlayMontage` (`self.Mesh`) "/Game/Animations/Melee/Montage_Unsheathing_Sword.Montage_Unsheathing_Sword")
    (:`OnCompleted`
      (`self.OnWeaponEquipped`))
    (:`OnNotifyBegin`
      ;; On the Montage Notify, Spawn the Weapon and attach it to the mesh Hand. Also SET the weapon actor variable.
      (switch `name` _notifyname
        (:`HoldSword`
          (bind _returnvalue (`|SpawnActorFromClass` "/Game/Weapons/BP_Weapon_Sword.BP_Weapon_Sword_C" (`self.GetTransform`) "Undefined" "MultiplyWithRoot" null null))
          (bind _output_get (set `self.WeaponActor` _returnvalue))
          (`self.K2_AttachToComponent` _output_get (`self.Mesh`) "hand_r_sword_socket" "SnapToTarget" "SnapToTarget" "SnapToTarget" true)
          ;; Finally, SET is wielding weapon to true
          (set `self.IsWieldingWeapon` true))))))

(event `/Game/Enemies/AI/BPI_EnemyAI.UnequipWeapon`
  ; Unequipp Weapon (Override) This event will be called by the BTT Unequip Weapon
  ;; Play Montage, and when completed, notify the BTT
  (bind _notifyname (`|PlayMontage` (`self.Mesh`) "/Game/Animations/Melee/Montage_Sheathing_Sword.Montage_Sheathing_Sword")
    (:`OnCompleted`
      (`self.OnWeaponUnequipped`))
    (:`OnNotifyBegin`
      ;; On the Montage Notify, destroy the Weapon
      (switch `name` _notifyname
        (:`DropSword`
          (`self.K2_DestroyActor` (`self.WeaponActor`))
          ;; Finally, SET is wielding weapon to false
          (set `self.IsWieldingWeapon` false))))))

(event `StartBlock`
  ; Blocking (Own logic) The Start Block event will be called by the BTT Melee Block. This task will expect a dispatch On Block Ended, which will be called by the End Block event
  ;; Blocking
  ;;; Stop movement, SET is blocking to true, SET Blocking State as Blocking, Play Montage
  (`MovementComponent.StopMovementImmediately` (`self.CharacterMovement`))
  (set `/Game/DamageSystem/BPC_DamageSystem.IsBlocking` true (`self.BPC_DamageSystem`))
  (set `self.BlockingState` "NewEnumerator1")
  (`|PlayMontage` (`self.Mesh`) "/Game/Animations/Melee/Montage_Sword_Block.Montage_Sword_Block"
    (:`OnCompleted`
      ;;; Call End Block (self)
      (`self.EndBlock` :!label _label_2))
    (:`OnInterrupted`
      ;;; The case where the Montage was interrupted AND the blocking state IS BlockedSuccessfully whil be covered by the Damage System. The Damage System Will dispatch the On Block event, which we will assign here
      (if (`|EnumInequality` (`self.BlockingState`) "NewEnumerator2")
        (goto _label_2)))))

(event `self.BPC_DamageSystem.OnBlocked`
  (params (CanBeParried :type Boolean))
  ; Blocking (Own logic) The Start Block event will be called by the BTT Melee Block. This task will expect a dispatch On Block Ended, which will be called by the End Block event
  ;; On Blocked (Dispatched by Damage System)
  ;;; SET Blocking Sate to Blocked Successfully
  (set `self.BlockingState` "NewEnumerator2")
  ;;; Play Montage
  (`|PlayMontage` (`self.Mesh`) "/Game/Animations/Melee/Montage_Sword_Block_React.Montage_Sword_Block_React"
    (:`OnCompleted`
      _)
    (:`OnInterrupted`
      _))
  ;;; Call End Block (self)
  (`self.EndBlock`))

(event `EndBlock`
  ; Blocking (Own logic) The Start Block event will be called by the BTT Melee Block. This task will expect a dispatch On Block Ended, which will be called by the End Block event
  ;; End Block
  ;;; SET is blocking to false, SET Blocking State to None
  (set `/Game/DamageSystem/BPC_DamageSystem.IsBlocking` false (`self.BPC_DamageSystem`))
  (set `self.BlockingState` "NewEnumerator0")
  ;;; Notify the BTT when complete
  (`self.OnBlockEnded`))

(fn `UserConstructionScript`
  (`parent.UserConstructionScript`))