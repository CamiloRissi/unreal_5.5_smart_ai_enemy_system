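; Attack component that gives its owning actor hitscan bullet and homing-style magic projectile attacks with team-aware damage.
; FireBullet line-traces for pawns and damages the first non-team hit, while MagicSpell spawns a targeted dark energy projectile that damages whatever it hits, without a team check, then signals attack end.
; Both report damage events for AI perception.
; A helper damages all non-team hits once each, tracking victims in an array.
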(event `FireBullet`
  (params (TraceStart :type "Vector Structure") (TraceEnd :type "Vector Structure") (DamageInfo :type "/Game/DamageSystem/S_DamageInfo Structure"))
  (bind (_outhits _returnvalue) (`KismetSystemLibrary.LineTraceMultiForObjects` TraceStart TraceEnd (`|MakeArray` "ObjectTypeQuery3" :!type "EObjectTypeQuery Enum") false (`|MakeArray` (`self.GetOwner`)) "ForDuration"))
  (if _returnvalue
    (bind _damagedactor (`self.DamageFirstNoneTeamMember` _outhits DamageInfo))
    (`AISense_Damage.ReportDamageEvent` _damagedactor (`self.GetOwner`) (`.Amount_2_369D13DA4D7F4B5016BB0BB08993A14F` (break `/Game/DamageSystem/S_DamageInfo` DamageInfo)) (`Actor.K2_GetActorLocation` (`self.GetOwner`)))))

(event `MagicSpell`
  (params (SpawnTransform :type "Transform Structure") (Target :type "Actor Object Reference") (DamageInfo :type "/Game/DamageSystem/S_DamageInfo Structure"))
  (bind _returnvalue (`|SpawnActorFromClass` "/Game/Projectiles/BP_Projectile_DarkEnergy.BP_Projectile_DarkEnergy_C" SpawnTransform "Undefined" "MultiplyWithRoot" (`self.GetOwner`) 1000.0 0.0 Target false null))
  (add `/Game/Projectiles/BP_Projectile_Base.OnProjectileImpact` _returnvalue (delegate `OnProjectileHit`))
  (`PrimitiveComponent.IgnoreActorWhenMoving` (`/Game/Projectiles/BP_Projectile_Base.BoxCollision` _returnvalue) (`self.GetOwner`) true))

(event `OnProjectileHit`
  (params (`Other Actor` :type "Actor Object Reference") (Hit :type "HitResult Structure"))
  (message `/Game/DamageSystem/BPI_Damagable.TakeDamage` `Other Actor` (stale `MagicSpell` DamageInfo) (`self.GetOwner`))
  (`AISense_Damage.ReportDamageEvent` `Other Actor` (`self.GetOwner`) (`.Amount_2_369D13DA4D7F4B5016BB0BB08993A14F` (break `/Game/DamageSystem/S_DamageInfo` (stale `MagicSpell` DamageInfo))) (`Actor.K2_GetActorLocation` (`self.GetOwner`)))
  (`self.OnAttackEnded`))

(fn `DamageAllNonTeamMemebers`
  (params (Hits :type "Array of HitResult Structure") (DamageInfo :type "/Game/DamageSystem/S_DamageInfo Structure"))
  (returns (ActorsDamaged :type "Array of Actor Object Reference"))
  (locals (ActorsDamagedSoFar :type "Array of Actor Object Reference"))
  (for _array_element Hits
    (bind (_bblockinghit _binitialoverlap _time _distance _location _impactpoint _normal _impactnormal _physmat _hitactor) (`GameplayStatics.BreakHitResult` _array_element))
    ; For Each Actor Hit
    ;; Check if hit actor is not on the same team
    (bind _teamnumber (message `/Game/DamageSystem/BPI_Damagable.GetTeamNumber` _hitactor))
    (bind _teamnumber_2 (message `/Game/DamageSystem/BPI_Damagable.GetTeamNumber` (`self.GetOwner`)))
    ;; Check if actor was already damaged
    (if (and (!= _teamnumber_2 _teamnumber) (not (`KismetArrayLibrary.Array_Contains` (`local.ActorsDamagedSoFar`) _hitactor)))
      ;; Call Take Damage on the Hit Actor and Add it to the ActorsDamagedSoFar Array
      (message `/Game/DamageSystem/BPI_Damagable.TakeDamage` _hitactor DamageInfo (`self.GetOwner`))
      (`KismetArrayLibrary.Array_AddUnique` (`local.ActorsDamagedSoFar`) _hitactor)))
  ; Return the damaged Actors
  (return (`local.ActorsDamagedSoFar`)))

(fn `DamageFirstNoneTeamMember`
  (params (Hits :type "Array of HitResult Structure") (DamageInfo :type "/Game/DamageSystem/S_DamageInfo Structure"))
  (returns (DamagedActor :type "Actor Object Reference"))
  ; For Each Actor Hit
  (for _array_element Hits
    (bind (_bblockinghit _binitialoverlap _time _distance _location _impactpoint _normal _impactnormal _physmat _hitactor) (`GameplayStatics.BreakHitResult` _array_element))
    ;; Check if hit actor is not on the same team
    (bind _teamnumber (message `/Game/DamageSystem/BPI_Damagable.GetTeamNumber` _hitactor))
    (bind _teamnumber_2 (message `/Game/DamageSystem/BPI_Damagable.GetTeamNumber` (`self.GetOwner`)))
    ;; Call Take Damage on the Hit Actor and break the loop
    (if (!= _teamnumber_2 _teamnumber)
      (message `/Game/DamageSystem/BPI_Damagable.TakeDamage` _hitactor DamageInfo (`self.GetOwner`))
      (`|ExecutionSequence`
        (:`then_0`
          (break))
        (:`then_1`
          (return _hitactor))))))